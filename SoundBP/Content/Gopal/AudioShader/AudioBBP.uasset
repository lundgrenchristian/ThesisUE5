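; Audio-reactive Blueprint that drives a material on its Cube from live spectral analysis of a player submix.
; BeginPlay creates a dynamic instance of the Balloon material and starts eight-band constant-Q analysis on the submix.
; Each analysis callback writes every band's clamped strength to a scalar parameter named by its one-based band number.
; Constant-Q NRT lookup, render-target and cube-scaling nodes are unwired leftovers.
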(event `self.ReceiveBeginPlay`
  (bind _returnvalue (`PrimitiveComponent.CreateDynamicMaterialInstance` (`self.Cube`) 0 "/Game/Gopal/AudioShader/Balloon.Balloon" "None"))
  (`KismetSystemLibrary.PrintString` "Hello")
  (`SoundSubmix.AddSpectralAnalysisDelegate` (`self.Player Submix`) (`AudioMixerBlueprintLibrary.MakeFullSpectrumSpectralAnalysisBandSettings` 8 40.0 10000.0) (delegate `CustomEvent_1`) 30.0 -40.0 true false 0.1 1.0)
  (`SoundSubmix.StartSpectralAnalysis` (`self.Player Submix`) "Large" "ConstantQ" "Blackman" 0.0 "PowerSpectrum"))

(event `CustomEvent_1`
  (params (Magnitude :type "Array of Float (double-precision) (by ref)"))
  (for (_array_element _array_index) Magnitude
    (set `self.BandNumber` _array_index)
    (bind _output_get (set `self.BandStrength` _array_element))
    (`MaterialInstanceDynamic.SetScalarParameterValue` (stale `self.ReceiveBeginPlay` _returnvalue) (`KismetStringLibrary.Conv_StringToName` (`KismetStringLibrary.Conv_IntToString` (+ _array_index 1))) (`KismetMathLibrary.FClamp` _output_get))))

(fn `UserConstructionScript`)